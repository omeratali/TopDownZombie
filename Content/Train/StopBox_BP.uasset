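; StopBox_BP is a trigger volume that halts the train at a stop for a while.
; On BeginPlay it finds the level's Spline_BP actor and stores a reference to it.
; When a Train_BP overlaps its box while that spline's Timeline is playing, it stops the Timeline, waits a fixed delay, then resumes it if still stopped.
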(event `self.ReceiveBeginPlay`
  (bind _returnvalue (`GameplayStatics.GetActorOfClass` "/Game/Train/Spline_BP.Spline_BP_C"))
  (bind _output_get (set `self.SplineRef` _returnvalue)))

(event `self.Box.OnComponentBeginOverlap`
  (params (OverlappedComponent :type "PrimitiveComponent Object Reference") (OtherActor :type "Actor Object Reference") (OtherComp :type "PrimitiveComponent Object Reference") (OtherBodyIndex :type Integer) (bFromSweep :type Boolean) (SweepResult :type "HitResult Structure (by ref)"))
  (cast `/Game/Train/Train_BP` OtherActor)
  (bind _timeline (`/Game/Train/Spline_BP.Timeline` (stale `self.ReceiveBeginPlay` _output_get)))
  (if (`TimelineComponent.IsPlaying` _timeline)
    (`TimelineComponent.Stop` _timeline)
    (`KismetSystemLibrary.Delay` 30.0)
    (if (not (`TimelineComponent.IsPlaying` _timeline))
      (`TimelineComponent.Play` _timeline))))

(fn `UserConstructionScript`)