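; Spline actor that moves the level's train along its spline path, starting automatically on BeginPlay.
; StartTrain finds the Train_BP actor and plays a Timeline whose track is lerped into a distance from zero to the spline's full length.
; Each update sets the train's world location and rotation from the spline at that distance.
; A StopBox_BP reference is also cached on BeginPlay but is not used here.
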(event `self.ReceiveBeginPlay`
  (bind _returnvalue (`GameplayStatics.GetActorOfClass` "/Game/Train/StopBox_BP.StopBox_BP_C"))
  (set `self.StopBox` _returnvalue)
  (`self.startTrain`))

(event `startTrain`
  (bind _spline (`self.Spline`))
  (bind _returnvalue (`GameplayStatics.GetActorOfClass` "/Game/Train/Train_BP.Train_BP_C"))
  (set `self.TrainRef` _returnvalue)
  (bind (_direction _newtrack_0) (`Timeline|Timeline`)
    (:`Update`
      (bind _returnvalue_2 (`KismetMathLibrary.Lerp` 0.0 (`SplineComponent.GetSplineLength` (`self.Spline`)) _newtrack_0))
      (`self.K2_SetActorLocationAndRotation` (`self.TrainRef`) (`SplineComponent.GetLocationAtDistanceAlongSpline` _spline _returnvalue_2 "World") (`SplineComponent.GetRotationAtDistanceAlongSpline` _spline _returnvalue_2 "World") false false))))

(fn `UserConstructionScript`)